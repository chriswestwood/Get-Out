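; Game state Blueprint that holds a level countdown and a randomly generated numeric key code.
; The Construction Script builds KeyNumbers by appending random digits to a string.
; UpdateTimer adds the supplied delta to LevelTimer while LevelStart is set and returns whether MaxLevelTime has been reached.
; GetTimeLeft returns the remaining time as a two-decimal string, or "GAME OVER" once it drops below zero.
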(event `self.ReceiveBeginPlay`)

(fn `GetTimeLeft`
  (returns (time :type String))
  (bind _returnvalue (- (`self.MaxLevelTime`) (`self.LevelTimer`)))
  (if (>= _returnvalue 0.0)
    (return (`KismetTextLibrary.Conv_TextToString` (`KismetTextLibrary.Conv_DoubleToText` _returnvalue "HalfToEven" false false 1 324 2 2)))
    (else
      (return "GAME OVER"))))

(fn `UpdateTimer`
  (params (delta :type "Float (double-precision)"))
  (returns (bIsGameOver :type Boolean))
  (if (`self.LevelStart`)
    (bind _output_get (set `self.LevelTimer` (+ delta (`self.LevelTimer`)))))
  (return (>= _output_get (`self.MaxLevelTime`))))

(fn `UserConstructionScript`
  (for _ (range 4)
    (set `self.KeyNumbers` (`KismetStringLibrary.Concat_StrStr` (`self.KeyNumbers`) (`KismetStringLibrary.Conv_IntToString` (`KismetMathLibrary.RandomInteger` 9))))))