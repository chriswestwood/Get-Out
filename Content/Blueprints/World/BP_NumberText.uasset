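; BP_NumberText is a world text actor that displays one character of the game mode's key numbers.
; On BeginPlay it gets the key number string from Bp_GameMode and shows the character at its KeyNumber index on its TextRender.
; ActivateSelf toggles visibility and, when activating, sets a lifespan so the actor is destroyed after the given time.
; A SetText function also allows the displayed text to be replaced directly.
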(event `self.ReceiveBeginPlay`
  (bind _asbp_game_mode (cast `/Game/Blueprints/Bp_GameMode` (`GameplayStatics.GetGameMode`)))
  (bind _keynums (`/Game/Blueprints/Bp_GameMode.GetKeyNums` _asbp_game_mode))
  (`TextRenderComponent.K2_SetText` (`self.TextRender`) (`KismetTextLibrary.Conv_StringToText` (`|GetArrayItem` (`KismetStringLibrary.GetCharacterArrayFromString` _keynums) (`self.KeyNumber`)))))

(event `/Game/Blueprints/World/Activateable.ActivateSelf`
  (params (isActive :type "Boolean (by ref)") (TIme :type Integer))
  (`self.SetActorHiddenInGame` (not isActive))
  (if isActive
    (`self.SetLifeSpan` (`KismetMathLibrary.Conv_IntToDouble` TIme))))

(fn `SetText`
  (params (NewText :type Text))
  (`TextRenderComponent.K2_SetText` (`self.TextRender`) NewText))

(fn `UserConstructionScript`)