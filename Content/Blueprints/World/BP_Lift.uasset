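; BP_Lift is a lift actor that moves vertically between numbered floors, and can also serve as the level's start lift.
; On BeginPlay it records its base location and, if floor height is zero, takes it from the Top component's relative Z.
; When active, MoveToFloor drives a Timeline that lerps the root to the target floor's height.
; If flagged as the start lift, it calls StartLevel on Bp_GameMode when the move finishes.
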(event `self.ReceiveBeginPlay`
  (if (== (`self.FloorHeight`) 0.0)
    (set `self.FloorHeight` (.z (`SceneComponent.RelativeLocation` (`self.top`)))))
  (set `self.Floor0Location` (`SceneComponent.RelativeLocation` (`self.DefaultSceneRoot`))))

(event `self.ReceiveTick`
  (params (DeltaSeconds :type "Float (single-precision)")))

(event `MoveToFloor`
  (params (Floor :type Integer))
  (if (`self.isActive`)
    (set `self.StartLocation` (`SceneComponent.RelativeLocation` (`self.DefaultSceneRoot`)))
    (set `self.EndLocation` (`KismetMathLibrary.MakeVector` (.x (`self.Floor0Location`)) (.y (`self.Floor0Location`)) (+ (* Floor (`self.FloorHeight`)) (.z (`self.Floor0Location`)))))
    (bind (_direction _alpha) (`Timeline|Timeline_0` :!via `PlayFromStart`)
      (:`Update`
        (`SceneComponent.K2_SetRelativeLocation` (`self.DefaultSceneRoot`) (`KismetMathLibrary.VLerp` (`self.StartLocation`) (`self.EndLocation`) _alpha) false false))
      (:`Finished`
        (if (`self.isStartLift`)
          (bind _asbp_game_mode (cast `/Game/Blueprints/Bp_GameMode` (`GameplayStatics.GetGameMode`)))
          (`/Game/Blueprints/Bp_GameMode.StartLevel` _asbp_game_mode))))))

(fn `UserConstructionScript`)